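; BP_Smasher_R is a moving smasher hazard that respawns the player on contact.
; On BeginPlay it stores its start location and plays a Timeline that lerps it up to 300 units along Y from that point.
; Overlapping its Box component casts the other actor to BP_FirstPersonCharacter and calls Respawn on it.
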(event OnComponentBeginOverlap(Box)
  (params (OverlappedComponent :type Primitive%20Component%20Object%20Reference) (OtherActor :type Actor%20Object%20Reference) (OtherComp :type Primitive%20Component%20Object%20Reference) (OtherBodyIndex :type Integer) (bFromSweep :type Boolean) (SweepResult :type Hit%20Result%20Structure%20%28by%20ref%29))
  (bind _asbp_first_person_character (Utilities|Casting|CastToBP_FirstPersonCharacter OtherActor))
  (Default|Respawn _asbp_first_person_character))

(event EventBeginPlay
  (Variables|Default|SetstartLoc (Transformation|GetActorLocation))
  (bind _newtrack_0 (Timeline|Timeline Play)
    (:Update
      (Transformation|SetActorRelativeLocation (Math|Vector|Lerp(Vector) (Variables|Default|GetstartLoc) (+ (Variables|Default|GetstartLoc) "0.000000,300.000000,0.000000") _newtrack_0)))))

(event Collision|EventActorBeginOverlap
  (params (OtherActor :type Actor%20Object%20Reference)))

(event EventTick
  (params (DeltaSeconds :type Float%20%28single-precision%29)))

(fn ConstructionScript)