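; BP_Door is a door actor that slides upward when opened and respawns the player on contact with its collider.
; OpenDoor turns off the actor's collision, then plays the DoorMovement timeline to lerp the Door component's relative location up along Z.
; Overlapping the Collider casts the other actor to BP_FirstPersonCharacter and calls its Respawn.
; BeginPlay stores the actor location in DoorLocation, which these graphs never read.
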(event OnComponentBeginOverlap(Collider)
  (params (OverlappedComponent :type Primitive%20Component%20Object%20Reference) (OtherActor :type Actor%20Object%20Reference) (OtherComp :type Primitive%20Component%20Object%20Reference) (OtherBodyIndex :type Integer) (bFromSweep :type Boolean) (SweepResult :type Hit%20Result%20Structure%20%28by%20ref%29))
  (bind _asbp_first_person_character (Utilities|Casting|CastToBP_FirstPersonCharacter OtherActor))
  (Default|Respawn _asbp_first_person_character))

(event Custom|OpenDoor
  (Collision|SetActorEnableCollision false)
  (bind _newtrack_0 (Timeline|Door%20Movement PlayFromStart)
    (:Update
      (Transformation|SetRelativeLocation (Variables|Default|GetDoor) (Math|Vector|Lerp(Vector) "0, 0, 0" "0.000000,0.000000,300.000000" _newtrack_0) false false))))

(event Collision|EventActorBeginOverlap
  (params (OtherActor :type Actor%20Object%20Reference)))

(event EventTick
  (params (DeltaSeconds :type Float%20%28single-precision%29)))

(event EventBeginPlay
  (Variables|Default|SetDoorLocation (Transformation|GetActorLocation)))

(fn ConstructionScript)