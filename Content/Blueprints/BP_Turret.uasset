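; BP_Turret is a prototype turret that switches between searching and targeting using the DetectionRadius overlap component.
; Any overlap sets EnemyDetected after a one-second delay, with no actor filtering, and end overlap clears it immediately.
; Tick reads that flag, either re-issuing the looping turret animation every frame while searching or running a visibility line trace whose result is unused.
; Both states only print debug text, with no aiming or firing logic.
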(event OnComponentBeginOverlap(DetectionRadius)
  (params (OverlappedComponent :type Primitive%20Component%20Object%20Reference) (OtherActor :type Actor%20Object%20Reference) (OtherComp :type Primitive%20Component%20Object%20Reference) (OtherBodyIndex :type Integer) (bFromSweep :type Boolean) (SweepResult :type Hit%20Result%20Structure%20%28by%20ref%29))
  (Utilities|FlowControl|Delay 1.0)
  (Development|PrintString "Detected!")
  (Variables|Default|SetEnemyDetected true))

(event OnComponentEndOverlap(DetectionRadius)
  (params (OverlappedComponent :type Primitive%20Component%20Object%20Reference) (OtherActor :type Actor%20Object%20Reference) (OtherComp :type Primitive%20Component%20Object%20Reference) (OtherBodyIndex :type Integer))
  (Variables|Default|SetEnemyDetected false))

(event EventBeginPlay
  (Collision|IgnoreActorwhenMoving (Variables|Default|GetDetectionRadius) self true)
  (Variables|Default|SetEnemyDetected false))

(event Collision|EventActorBeginOverlap
  (params (OtherActor :type Actor%20Object%20Reference)))

(event EventTick
  (params (DeltaSeconds :type Float%20%28single-precision%29))
  (if (Variables|Default|GetEnemyDetected)
    (Development|PrintString "Targeting Enemy")
    (Collision|LineTraceByChannel "0, 0, 0" "0, 0, 0" "TraceTypeQuery1" false 0 "None")
    (else
      (Components|Animation|PlayAnimation (Variables|Default|Getconnector_Material_001_0) "/Game/Fab/Sci-fi_turret/sci_fi_turret/SkeletalMeshes/sci_fi_turret_Anim.sci_fi_turret_Anim" true)
      (Development|PrintString "Searching for Enemy"))))

(fn ConstructionScript)